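; Player character Blueprint that adds keyboard hotkeys, apparently for testing, to control game speed and trigger a fire effect.
; Add and Subtract step global time dilation up and down between stopped, SlowTime and OriginTime by checking the current value.
; T spawns the NS_Body_Fire Niagara system attached to the mesh's right weapon socket.
; BeginPlay, overlap and Tick are disabled parent-call stubs, and a TriggerActionBlueprint call is left unconnected.
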(event `Key|Add`
  (params (Key :type "Key Structure"))
  (:`Pressed`
    (if (== (`GameplayStatics.GetGlobalTimeDilation`) 0.0)
      (`GameplayStatics.SetGlobalTimeDilation` (`self.SlowTime`))
      (else
        (`GameplayStatics.SetGlobalTimeDilation` (`self.OriginTime`))))))

(event `Key|Subtract`
  (params (Key :type "Key Structure"))
  (bind _slowtime (`self.SlowTime`))
  (:`Pressed`
    (if (== (`GameplayStatics.GetGlobalTimeDilation`) _slowtime)
      (`GameplayStatics.SetGlobalTimeDilation` 0.0)
      (else
        (`GameplayStatics.SetGlobalTimeDilation` _slowtime)))))

(event `Key|T`
  (params (Key :type "Key Structure"))
  (:`Pressed`
    (`NiagaraFunctionLibrary.SpawnSystemAttached` "/Game/CharacterBodyFX/FX/Fire/NS_Body_Fire.NS_Body_Fire" (`self.Mesh`) "Weapon-r" (0.0 0.0 0.0) (struct) "KeepRelativeOffset")))

(fn `UserConstructionScript`
  (`parent.UserConstructionScript`))